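; Interactable door with closed, semi-open, opened and locked states, driven by the first-person character's Interact event.
; Press opens or closes it; hold cracks it slightly, and releasing swings a semi-open door fully.
; Timelines lerp Scene yaw according to OpeningDirection, then store rotation and state.
; Side trigger boxes let a running character burst it open in the matching direction; peeking and locked-door feedback are empty stubs.
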(event `/Game/Blueprint/Other/BPI_Interact.Interact`
  (params (HitComponent :type "PrimitiveComponent Object Reference") (Character :type "Character Object Reference") (InteractionType :type "/Game/Blueprint/Character/E_InteractionType Enum" :default "NewEnumerator0"))
  (cast `/Game/Blueprint/Character/BP_FirstPersonCharacter` Character)
  (switch `/Game/Blueprint/Character/E_InteractionType` InteractionType
    (:`NewEnumerator0`
      (switch `/Game/Blueprint/Interactible/OtherThing/E_DoorState` (`self.DoorState`)
        (:`NewEnumerator0`
          (`self.OpenDoor` (`self.OpenRightRot`) (`self.OpenLeftRot`) "NewEnumerator2" :!label _label))
        (:`NewEnumerator1`
          (goto _label))
        (:`NewEnumerator2`
          (`self.CloseDoor`))
        (:`NewEnumerator3`
          (`self.TryOpenDoor`))))
    (:`NewEnumerator1`
      (switch `/Game/Blueprint/Interactible/OtherThing/E_DoorState` (`self.DoorState`)
        (:`NewEnumerator0`
          (`|ExecutionSequence`
            (:`then_0`
              (`self.OpenDoor` (`self.SlightOpenRightRot`) (`self.SlightOpenLeftRot`) "NewEnumerator1"))
            (:`then_1`
              (`self.SemiOpenDoorPeaking` :!label _label_2))))
        (:`NewEnumerator1`
          (goto _label_2))
        (:`NewEnumerator3`
          (`self.TryOpenDoor`))))
    (:`NewEnumerator2`
      (switch `/Game/Blueprint/Interactible/OtherThing/E_DoorState` (`self.DoorState`)
        (:`NewEnumerator1`
          (`self.OpenDoor` (`self.OpenRightRot`) (`self.OpenLeftRot`) "NewEnumerator2"))))))

(event `OpenDoor`
  (params (RightOpenRot :type "Rotator Structure") (LeftOpenRot :type "Rotator Structure") (DoorState :type "/Game/Blueprint/Interactible/OtherThing/E_DoorState Enum" :default "NewEnumerator0"))
  (bind (_currentrot_roll _currentrot_pitch _currentrot_yaw) (`KismetMathLibrary.BreakRotator` (`self.CurrentRot`)))
  (bind (_currentrot_roll_2 _currentrot_pitch_2 _currentrot_yaw_2) (`KismetMathLibrary.BreakRotator` (`self.CurrentRot`)))
  (bind (_direction _opening_closing) (`Timeline|OpeningDoor` :!label _label_3)
    (:`Update`
      (switch `/Game/Blueprint/Interactible/OtherThing/E_OpeningSide` (`self.OpeningDirection`)
        (:`NewEnumerator0`
          (`SceneComponent.K2_SetRelativeRotation` (`self.Scene`) (`KismetMathLibrary.MakeRotator` _currentrot_roll _currentrot_pitch (`KismetMathLibrary.Lerp` _currentrot_yaw (.yaw RightOpenRot) _opening_closing)) false false))
        (:`NewEnumerator1`
          (`SceneComponent.K2_SetRelativeRotation` (`self.Scene`) (`KismetMathLibrary.MakeRotator` _currentrot_roll_2 _currentrot_pitch_2 (`KismetMathLibrary.Lerp` _currentrot_yaw_2 (.yaw LeftOpenRot) _opening_closing)) false false))))
    (:`Finished`
      (set `self.CurrentRot` (`SceneComponent.RelativeRotation` (`self.Scene`)))
      (set `self.DoorState` DoorState)
      (goto _label_3 :!via `SetNewTime`))))

(event `CloseDoor`
  (bind (_currentrot_roll _currentrot_pitch _currentrot_yaw) (`KismetMathLibrary.BreakRotator` (`self.CurrentRot`)))
  (bind (_closedrot_roll _closedrot_pitch _closedrot_yaw) (`KismetMathLibrary.BreakRotator` (`self.ClosedRot`)))
  (bind (_direction _opening_closing) (`Timeline|ClosingDoor` :!label _label_4)
    (:`Update`
      (`SceneComponent.K2_SetRelativeRotation` (`self.Scene`) (`KismetMathLibrary.MakeRotator` _currentrot_roll _currentrot_pitch (`KismetMathLibrary.Lerp` _currentrot_yaw _closedrot_yaw _opening_closing)) false false))
    (:`Finished`
      (set `self.CurrentRot` (`SceneComponent.RelativeRotation` (`self.Scene`)))
      (set `self.DoorState` "NewEnumerator0")
      (goto _label_4 :!via `SetNewTime`))))

(event `SemiOpenDoorPeaking`)

(event `self.BoxLeft.OnComponentBeginOverlap`
  (params (OverlappedComponent :type "PrimitiveComponent Object Reference") (OtherActor :type "Actor Object Reference") (OtherComp :type "PrimitiveComponent Object Reference") (OtherBodyIndex :type Integer) (bFromSweep :type Boolean) (SweepResult :type "HitResult Structure (by ref)"))
  (bind (_openrightrot_roll _openrightrot_pitch _openrightrot_yaw) (`KismetMathLibrary.BreakRotator` (`self.OpenRightRot`)))
  (bind (_currentrot_roll _currentrot_pitch _currentrot_yaw) (`KismetMathLibrary.BreakRotator` (`self.CurrentRot`)))
  ; Allow character to push door quickly when running (door can only be opened on the right direction (can be changed depending on video game choices)
  (bind _asbp_first_person_character (cast `/Game/Blueprint/Character/BP_FirstPersonCharacter` OtherActor))
  (if (`BlueprintGameplayTagLibrary.HasTag` (`/Game/Blueprint/Character/BP_FirstPersonCharacter.GameplayTags` _asbp_first_person_character) (struct :`TagName` "Movement.Running") true)
    (switch `/Game/Blueprint/Interactible/OtherThing/E_DoorState` (`self.DoorState`)
      (:`NewEnumerator0`
        (bind (_direction _quickdooropening) (`Timeline|QuickDoorOpeningRight` :!label _label_5)
          (:`Update`
            (switch `/Game/Blueprint/Interactible/OtherThing/E_OpeningSide` (`self.OpeningDirection`)
              (:`NewEnumerator0`
                (`SceneComponent.K2_SetRelativeRotation` (`self.Scene`) (`KismetMathLibrary.MakeRotator` _currentrot_roll _currentrot_pitch (`KismetMathLibrary.Lerp` _currentrot_yaw _openrightrot_yaw _quickdooropening)) false false))))
          (:`Finished`
            (set `self.CurrentRot` (`SceneComponent.RelativeRotation` (`self.Scene`)))
            (set `self.DoorState` "NewEnumerator2"))))
      (:`NewEnumerator1`
        (goto _label_5)))))

(event `TryOpenDoor`
  ;[0.6875 0.2449 0 0.5] Add Animation of character trying to open door + sound
)

(event `self.BoxRight.OnComponentBeginOverlap`
  (params (OverlappedComponent :type "PrimitiveComponent Object Reference") (OtherActor :type "Actor Object Reference") (OtherComp :type "PrimitiveComponent Object Reference") (OtherBodyIndex :type Integer) (bFromSweep :type Boolean) (SweepResult :type "HitResult Structure (by ref)"))
  (bind (_currentrot_roll _currentrot_pitch _currentrot_yaw) (`KismetMathLibrary.BreakRotator` (`self.CurrentRot`)))
  (bind (_openleftrot_roll _openleftrot_pitch _openleftrot_yaw) (`KismetMathLibrary.BreakRotator` (`self.OpenLeftRot`)))
  ; Allow character to push door quickly when running (door can only be opened on the right direction (can be changed depending on video game choices)
  (bind _asbp_first_person_character (cast `/Game/Blueprint/Character/BP_FirstPersonCharacter` OtherActor))
  (if (`BlueprintGameplayTagLibrary.HasTag` (`/Game/Blueprint/Character/BP_FirstPersonCharacter.GameplayTags` _asbp_first_person_character) (struct :`TagName` "Movement.Running") true)
    (switch `/Game/Blueprint/Interactible/OtherThing/E_DoorState` (`self.DoorState`)
      (:`NewEnumerator0`
        (bind (_direction _quickdooropening) (`Timeline|QuickDoorOpeningLeft` :!label _label_6)
          (:`Update`
            (switch `/Game/Blueprint/Interactible/OtherThing/E_OpeningSide` (`self.OpeningDirection`)
              (:`NewEnumerator1`
                (`SceneComponent.K2_SetRelativeRotation` (`self.Scene`) (`KismetMathLibrary.MakeRotator` _currentrot_roll _currentrot_pitch (`KismetMathLibrary.Lerp` _currentrot_yaw _openleftrot_yaw _quickdooropening)) false false))))
          (:`Finished`
            (set `self.CurrentRot` (`SceneComponent.RelativeRotation` (`self.Scene`)))
            (set `self.DoorState` "NewEnumerator2"))))
      (:`NewEnumerator1`
        (goto _label_6)))))

(fn `UserConstructionScript`)